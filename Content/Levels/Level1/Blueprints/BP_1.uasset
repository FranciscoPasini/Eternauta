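; BP_1 is a Level 1 interaction trigger that lets the player travel to the level Nivel2.
; When the third-person character enters its Box, it enables input for the first player controller and shows a BPI_Interaction widget.
; While input is enabled, the IA_Action input opens Nivel2 by object reference.
; Leaving the Box disables input and removes the widget.
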(event `EnhancedInput|/Game/ThirdPerson/Input/Actions/IA_Action`
  (params (ActionValue :type Boolean) (ElapsedSeconds :type "Float (double-precision)") (TriggeredSeconds :type "Float (double-precision)") (InputAction :type "InputAction Object Reference" :default "/Game/ThirdPerson/Input/Actions/IA_Action.IA_Action"))
  ;[1 0.8366 0] Evento de pasar de escena
  (:`Triggered`
    (`GameplayStatics.OpenLevelBySoftObjectPtr` "/Game/Levels/Level2/Nivel2.Nivel2")))

(event `self.Box.OnComponentBeginOverlap`
  (params (OverlappedComponent :type "PrimitiveComponent Object Reference") (OtherActor :type "Actor Object Reference") (OtherComp :type "PrimitiveComponent Object Reference") (OtherBodyIndex :type Integer) (bFromSweep :type Boolean) (SweepResult :type "HitResult Structure (by ref)"))
  ;[0 0.06418 1] El jugador puede interactuar/canvas de interaccion
  (cast `/Game/ThirdPerson/Blueprints/BP_ThirdPersonCharacter` OtherActor)
  (`self.EnableInput` (`GameplayStatics.GetPlayerController` 0))
  (bind _returnvalue (`|CreateWidget` "/Game/Levels/Level2/BluePrints/BPI_Interaction.BPI_Interaction_C"))
  (`UserWidget.AddToViewport` _returnvalue 0))

(event `self.Box.OnComponentEndOverlap`
  (params (OverlappedComponent :type "PrimitiveComponent Object Reference") (OtherActor :type "Actor Object Reference") (OtherComp :type "PrimitiveComponent Object Reference") (OtherBodyIndex :type Integer))
  ;[0 1 0.0173] Deja de interactuar
  (cast `/Game/ThirdPerson/Blueprints/BP_ThirdPersonCharacter` OtherActor)
  (`self.DisableInput` (`GameplayStatics.GetPlayerController` 0))
  (`Widget.RemoveFromParent` (stale `self.Box.OnComponentBeginOverlap` _returnvalue)))

(fn `UserConstructionScript`)