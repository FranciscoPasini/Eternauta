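; BPAI is a Level 4 enemy pawn that roams at random and hunts the player, opening level Nivel4 when it catches them.
; From BeginPlay, it chains moves to random reachable points around itself.
; Seeing any pawn through PawnSensing sends it after player 0, whom it destroys on arrival.
; A one-second retriggerable delay returns it to wandering once sightings stop.
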(event `self.ReceiveBeginPlay`
  (`self.Goto`))

(event `Goto`
  (`|AIMoveTo` self (`NavigationSystemV1.K2_GetRandomReachablePointInRadius` (`self.K2_GetActorLocation`) 2500.0 null null) null
    (:`OnSuccess`
      (`self.Goto`))))

(event `self.PawnSensing.OnSeePawn`
  (params (Pawn :type "Pawn Object Reference"))
  (`|ExecutionSequence`
    (:`then_0`
      (`|AIMoveTo` self (0.0 0.0 0.0) (`GameplayStatics.GetPlayerPawn` 0)
        (:`OnSuccess`
          (`self.K2_DestroyActor` (`GameplayStatics.GetPlayerPawn` 0))
          (`GameplayStatics.OpenLevel` "Nivel4"))))
    (:`then_1`
      (`KismetSystemLibrary.RetriggerableDelay` 1.0)
      (`self.Goto`))))

(fn `UserConstructionScript`)