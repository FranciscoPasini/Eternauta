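; Keycard-locked red door in Level 2 that swings when the player interacts with it.
; A box overlap checks the character's KeyCard flag, then either enables input and shows the interaction widget or shows a missing-keycard widget.
; IA_Action plays a push montage and door sound, then a timeline rotates the door's yaw toward CloseDoor and removes the prompt.
; Leaving the box disables input and clears both widgets.
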(event `self.Box.OnComponentBeginOverlap`
  (params (OverlappedComponent :type "PrimitiveComponent Object Reference") (OtherActor :type "Actor Object Reference") (OtherComp :type "PrimitiveComponent Object Reference") (OtherBodyIndex :type Integer) (bFromSweep :type Boolean) (SweepResult :type "HitResult Structure (by ref)"))
  ;[1 0.01025 0.823] Verifica que el jugador este cercca y tenga la keycard
  (bind _asbp_third_person_character (cast `/Game/ThirdPerson/Blueprints/BP_ThirdPersonCharacter` OtherActor))
  (if (`/Game/ThirdPerson/Blueprints/BP_ThirdPersonCharacter.KeyCard` _asbp_third_person_character)
    ;[1 0.7456 0] El jugador puede abrir la puerta/canvas de interaccion
    (`self.EnableInput` (`GameplayStatics.GetPlayerController` 0))
    (bind _returnvalue (`|CreateWidget` "/Game/Levels/Level2/BluePrints/BPI_Interaction.BPI_Interaction_C"))
    (`UserWidget.AddToViewport` _returnvalue 0)
    (else
      (bind _returnvalue_2 (`|CreateWidget` "/Game/Levels/Level2/BluePrints/BPI_MissingKeycard.BPI_MissingKeycard_C"))
      (`UserWidget.AddToViewport` _returnvalue_2 0)
      ;[1 1 1] El jugador tiene la tarjeta
      (if (`/Game/ThirdPerson/Blueprints/BP_ThirdPersonCharacter.KeyCard` _asbp_third_person_character)
        (`Widget.RemoveFromParent` _returnvalue_2)))))

(event `EnhancedInput|/Game/ThirdPerson/Input/Actions/IA_Action`
  (params (ActionValue :type Boolean) (ElapsedSeconds :type "Float (double-precision)") (TriggeredSeconds :type "Float (double-precision)") (InputAction :type "InputAction Object Reference" :default "/Game/ThirdPerson/Input/Actions/IA_Action.IA_Action"))
  (:`Triggered`
    (`|ExecutionSequence`
      (:`then_0`
        (`Character.PlayAnimMontage` (`GameplayStatics.GetPlayerCharacter` 0) "/Game/DownloadedAssets/RamsterZ_FreeAnims_Volume1/AnimationSequence/Paired/push.push" 1.0 "None"))
      (:`then_1`
        ;[0.2534 1 0] Sonido al cerrarse
        (`GameplayStatics.PlaySoundAtLocation` "/Game/Audio/close-door-sound-247450.close-door-sound-247450" (`self.K2_GetActorLocation`) (struct) 1.0 1.0 0.0 null null null null))
      (:`then_2`
        ;[0 0.7495 1] Evento de cerrar puerta
        (bind (_direction _doorrotation) (`Timeline|Rotation`)
          (:`Update`
            (`SceneComponent.K2_SetRelativeRotation` (`self.Door`) (`KismetMathLibrary.MakeRotator` 0.0 0.0 (`KismetMathLibrary.Lerp` 0.0 (`self.CloseDoor`) _doorrotation)) false false)
            (`Widget.RemoveFromParent` (stale `self.Box.OnComponentBeginOverlap` _returnvalue))))))))

(event `self.Box.OnComponentEndOverlap`
  (params (OverlappedComponent :type "PrimitiveComponent Object Reference") (OtherActor :type "Actor Object Reference") (OtherComp :type "PrimitiveComponent Object Reference") (OtherBodyIndex :type Integer))
  ;[0 1 0.1013] deja de interactuar
  (cast `/Game/ThirdPerson/Blueprints/BP_ThirdPersonCharacter` OtherActor)
  (`self.DisableInput` (`GameplayStatics.GetPlayerController` 0))
  (`Widget.RemoveFromParent` (stale `self.Box.OnComponentBeginOverlap` _returnvalue_2))
  (`Widget.RemoveFromParent` (stale `self.Box.OnComponentBeginOverlap` _returnvalue)))

(fn `UserConstructionScript`)