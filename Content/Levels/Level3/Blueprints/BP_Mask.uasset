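; BP_Mask is a collectible mask in Level 3 that removes the snow damage when picked up.
; Overlapping its box enables input and shows a pickup prompt widget for the third-person character; leaving reverses both.
; The action key plays a montage and sound, inserts true into the character's MaskBool at MaskValue, and destroys the mask.
; It then destroys the PainCausingVolume returned by GetActorOfClass.
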(event `EnhancedInput|/Game/ThirdPerson/Input/Actions/IA_Action`
  (params (ActionValue :type Boolean) (ElapsedSeconds :type "Float (double-precision)") (TriggeredSeconds :type "Float (double-precision)") (InputAction :type "InputAction Object Reference" :default "/Game/ThirdPerson/Input/Actions/IA_Action.IA_Action"))
  ;[1 1 1] Collect
  (:`Triggered`
    (`|ExecutionSequence`
      (:`then_0`
        ;[1 1 1] Animation of Collect
        (`Character.PlayAnimMontage` (`GameplayStatics.GetPlayerCharacter` 0) "/Game/DownloadedAssets/RamsterZ_FreeAnims_Volume1/AnimationSequence/Paired/push.push" 1.0 "None"))
      (:`then_1`
        ;;[1 1 1] Sound of Collect
        (`GameplayStatics.PlaySoundAtLocation` "/Game/Audio/item-picked.item-picked" (`self.K2_GetActorLocation`) (struct) 1.0 1.0 0.0 null null null null))
      (:`then_2`
        (`KismetArrayLibrary.Array_Insert` (`/Game/ThirdPerson/Blueprints/BP_ThirdPersonCharacter.MaskBool` (stale `self.Box.OnComponentBeginOverlap` _asbp_third_person_character)) true (`self.MaskValue`))
        (`self.K2_DestroyActor`))
      (:`then_3`
        ;[1 1 1] Se borra el daño de la nieve
        (bind _returnvalue (`GameplayStatics.GetActorOfClass` "/Script/Engine.PainCausingVolume"))
        (`self.K2_DestroyActor` _returnvalue)))))

(event `self.Box.OnComponentBeginOverlap`
  (params (OverlappedComponent :type "PrimitiveComponent Object Reference") (OtherActor :type "Actor Object Reference") (OtherComp :type "PrimitiveComponent Object Reference") (OtherBodyIndex :type Integer) (bFromSweep :type Boolean) (SweepResult :type "HitResult Structure (by ref)"))
  ;[1 1 1] Box Collider of the Mask
  (bind _asbp_third_person_character (cast `/Game/ThirdPerson/Blueprints/BP_ThirdPersonCharacter` OtherActor))
  (`self.EnableInput` (`GameplayStatics.GetPlayerController` 0))
  (bind _returnvalue (`|CreateWidget` "/Game/Levels/Level3/Interfaces/BPI_PickUpMask.BPI_PickUpMask_C"))
  (`UserWidget.AddToViewport` _returnvalue 0))

(event `self.Box.OnComponentEndOverlap`
  (params (OverlappedComponent :type "PrimitiveComponent Object Reference") (OtherActor :type "Actor Object Reference") (OtherComp :type "PrimitiveComponent Object Reference") (OtherBodyIndex :type Integer))
  ;[1 1 1] Box Collider of the Mask
  ;;[1 1 1] When Leave
  (cast `/Game/ThirdPerson/Blueprints/BP_ThirdPersonCharacter` OtherActor)
  (`self.DisableInput` (`GameplayStatics.GetPlayerController` 0))
  (`Widget.RemoveFromParent` (stale `self.Box.OnComponentBeginOverlap` _returnvalue)))

(fn `UserConstructionScript`)