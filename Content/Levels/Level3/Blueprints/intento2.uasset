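; Level 3 exit trigger that lets a player holding the required keycard travel to Nivel4.
; On box overlap, it loops the character's KeyCard array for a true entry at index MaskCollected, then enables input and shows the interaction widget; pressing E opens the level.
; Each non-matching entry creates a cannot-escape widget, removed immediately by a nested loop if the card is held.
; Leaving the box disables input and removes the stored widgets.
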(event `self.Box.OnComponentBeginOverlap`
  (params (OverlappedComponent :type "PrimitiveComponent Object Reference") (OtherActor :type "Actor Object Reference") (OtherComp :type "PrimitiveComponent Object Reference") (OtherBodyIndex :type Integer) (bFromSweep :type Boolean) (SweepResult :type "HitResult Structure (by ref)"))
  ;[1 0.01025 0.823] Verifica que el jugador este cercca y tenga la keycard
  (bind _asbp_third_person_character (cast `/Game/ThirdPerson/Blueprints/BP_ThirdPersonCharacter` OtherActor))
  (for (_array_element _array_index) (`/Game/ThirdPerson/Blueprints/BP_ThirdPersonCharacter.KeyCard` _asbp_third_person_character)
    (if (and _array_element (== _array_index (`self.MaskCollected`)))
      ;[1 0.7456 0] El jugador puede abrir la puerta/canvas de interaccion
      (`self.EnableInput` (`GameplayStatics.GetPlayerController` 0))
      (bind _returnvalue (`|CreateWidget` "/Game/Levels/Level2/BluePrints/BPI_Interaction.BPI_Interaction_C"))
      (`UserWidget.AddToViewport` _returnvalue 0)
      (else
        (bind _returnvalue_2 (`|CreateWidget` "/Game/Levels/Level3/Interfaces/BPI_CanNotEscape.BPI_CanNotEscape_C"))
        (`UserWidget.AddToViewport` _returnvalue_2 0)
        ;[1 1 1] El jugador tiene la tarjeta
        (for (_array_element_2 _array_index_2) (`/Game/ThirdPerson/Blueprints/BP_ThirdPersonCharacter.KeyCard` _asbp_third_person_character)
          (if (and _array_element_2 (== _array_index_2 (`self.MaskCollected`)))
            (`Widget.RemoveFromParent` _returnvalue_2)))))))

(event `Key|E`
  (params (Key :type "Key Structure"))
  (:`Pressed`
    (`GameplayStatics.OpenLevel` "Nivel4")
    (`Widget.RemoveFromParent` (stale `self.Box.OnComponentBeginOverlap` _returnvalue))))

(event `self.Box.OnComponentEndOverlap`
  (params (OverlappedComponent :type "PrimitiveComponent Object Reference") (OtherActor :type "Actor Object Reference") (OtherComp :type "PrimitiveComponent Object Reference") (OtherBodyIndex :type Integer))
  ;[0 1 0.1013] deja de interactuar
  (cast `/Game/ThirdPerson/Blueprints/BP_ThirdPersonCharacter` OtherActor)
  (`self.DisableInput` (`GameplayStatics.GetPlayerController` 0))
  (`Widget.RemoveFromParent` (stale `self.Box.OnComponentBeginOverlap` _returnvalue))
  (`Widget.RemoveFromParent` (stale `self.Box.OnComponentBeginOverlap` _returnvalue_2)))

(fn `UserConstructionScript`)