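; Level exit door that lets the player advance to Nivel4 only when carrying the required mask.
; On box overlap, it loops through the character's MaskBool array; a true entry at MaskCollected enables door input and shows BPI_GoOutside.
; Each other entry spawns BPI_CanNotEscape, removed immediately if a nested loop finds the mask.
; IA_Action opens the level, while leaving the box disables input and removes the prompts.
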(event `self.Box.OnComponentBeginOverlap`
  (params (OverlappedComponent :type "PrimitiveComponent Object Reference") (OtherActor :type "Actor Object Reference") (OtherComp :type "PrimitiveComponent Object Reference") (OtherBodyIndex :type Integer) (bFromSweep :type Boolean) (SweepResult :type "HitResult Structure (by ref)"))
  ;[1 0 0.7838] Verifica que el jugador este cerca y que tenga la mascara
  (bind _asbp_third_person_character (cast `/Game/ThirdPerson/Blueprints/BP_ThirdPersonCharacter` OtherActor))
  (for (_array_element _array_index) (`/Game/ThirdPerson/Blueprints/BP_ThirdPersonCharacter.MaskBool` _asbp_third_person_character)
    (if (and _array_element (== _array_index (`self.MaskCollected`)))
      ;[1 0.8688 0] El jugador puede abrir la puerta/canvas de interaccion
      (`self.EnableInput` (`GameplayStatics.GetPlayerController` 0))
      (bind _returnvalue (`|CreateWidget` "/Game/Levels/Level3/Interfaces/BPI_GoOutside.BPI_GoOutside_C"))
      (`UserWidget.AddToViewport` _returnvalue 0)
      (else
        (bind _returnvalue_2 (`|CreateWidget` "/Game/Levels/Level3/Interfaces/BPI_CanNotEscape.BPI_CanNotEscape_C"))
        (`UserWidget.AddToViewport` _returnvalue_2 0)
        ;[1 1 1] El jugador tiene la máscara
        (for (_array_element_2 _array_index_2) (`/Game/ThirdPerson/Blueprints/BP_ThirdPersonCharacter.MaskBool` _asbp_third_person_character)
          (if (and _array_element_2 (== _array_index_2 (`self.MaskCollected`)))
            (`Widget.RemoveFromParent` _returnvalue_2)))))))

(event `EnhancedInput|/Game/ThirdPerson/Input/Actions/IA_Action`
  (params (ActionValue :type Boolean) (ElapsedSeconds :type "Float (double-precision)") (TriggeredSeconds :type "Float (double-precision)") (InputAction :type "InputAction Object Reference" :default "/Game/ThirdPerson/Input/Actions/IA_Action.IA_Action"))
  ;[0 0.6256 1] evento de pasar nivel
  (:`Triggered`
    (`GameplayStatics.OpenLevelBySoftObjectPtr` "/Game/Levels/Level4/Nivel4.Nivel4")
    (`Widget.RemoveFromParent` (stale `self.Box.OnComponentBeginOverlap` _returnvalue))))

(event `self.Box.OnComponentEndOverlap`
  (params (OverlappedComponent :type "PrimitiveComponent Object Reference") (OtherActor :type "Actor Object Reference") (OtherComp :type "PrimitiveComponent Object Reference") (OtherBodyIndex :type Integer))
  ;[0 1 0.1091] se aleja de la puerta
  (cast `/Game/ThirdPerson/Blueprints/BP_ThirdPersonCharacter` OtherActor)
  (`self.DisableInput` (`GameplayStatics.GetPlayerController` 0))
  (`Widget.RemoveFromParent` (stale `self.Box.OnComponentBeginOverlap` _returnvalue_2))
  (`Widget.RemoveFromParent` (stale `self.Box.OnComponentBeginOverlap` _returnvalue)))

(fn `UserConstructionScript`)