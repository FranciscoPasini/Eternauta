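; BP_KeycardDoor is a door that the player can open only when holding the keycard matching its KeycardValue.
; Box overlap scans the character's KeyCard array by index, enabling input with an Interaction widget on a match and handling a MissingKeycard widget otherwise.
; Pressing E plays the Rotation timeline, lerping door yaw from closed to open.
; Leaving the box disables input, removes widgets and reverses the timeline to close it.
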(event `self.Box.OnComponentBeginOverlap`
  (params (OverlappedComponent :type "PrimitiveComponent Object Reference") (OtherActor :type "Actor Object Reference") (OtherComp :type "PrimitiveComponent Object Reference") (OtherBodyIndex :type Integer) (bFromSweep :type Boolean) (SweepResult :type "HitResult Structure (by ref)"))
  (bind _asbp_third_person_character (cast `/Game/ThirdPerson/Blueprints/BP_ThirdPersonCharacter` OtherActor))
  (for (_array_element _array_index) (`/Game/ThirdPerson/Blueprints/BP_ThirdPersonCharacter.KeyCard` _asbp_third_person_character)
    (if (and _array_element (== _array_index (`self.KeycardValue`)))
      (`self.EnableInput` (`GameplayStatics.GetPlayerController` 0))
      (bind _returnvalue (`|CreateWidget` "/Game/BluePrints/Interaction.Interaction_C"))
      (`UserWidget.AddToViewport` _returnvalue 0)
      (else
        (bind _returnvalue_2 (`|CreateWidget` "/Game/BluePrints/MissingKeycard.MissingKeycard_C"))
        (`UserWidget.AddToViewport` _returnvalue_2 0)
        (for (_array_element_2 _array_index_2) (`/Game/ThirdPerson/Blueprints/BP_ThirdPersonCharacter.KeyCard` _asbp_third_person_character)
          (if (and _array_element_2 (== _array_index_2 (`self.KeycardValue`)))
            (`Widget.RemoveFromParent` _returnvalue_2)))))))

(event `Key|E`
  (params (Key :type "Key Structure"))
  (:`Pressed`
    (bind (_direction _doorrotation) (`Timeline|Rotation` :!label _label)
      (:`Update`
        (`SceneComponent.K2_SetRelativeRotation` (`self.Door`) (`KismetMathLibrary.MakeRotator` 0.0 0.0 (`KismetMathLibrary.Lerp` (`self.DoorClosed`) (`self.DoorOpen`) _doorrotation)) false false)
        (`Widget.RemoveFromParent` (stale `self.Box.OnComponentBeginOverlap` _returnvalue))))))

(event `self.Box.OnComponentEndOverlap`
  (params (OverlappedComponent :type "PrimitiveComponent Object Reference") (OtherActor :type "Actor Object Reference") (OtherComp :type "PrimitiveComponent Object Reference") (OtherBodyIndex :type Integer))
  (cast `/Game/ThirdPerson/Blueprints/BP_ThirdPersonCharacter` OtherActor)
  (`self.DisableInput` (`GameplayStatics.GetPlayerController` 0))
  (`Widget.RemoveFromParent` (stale `self.Box.OnComponentBeginOverlap` _returnvalue))
  (`Widget.RemoveFromParent` (stale `self.Box.OnComponentBeginOverlap` _returnvalue_2))
  (goto _label :!via `Reverse`))

(fn `UserConstructionScript`)